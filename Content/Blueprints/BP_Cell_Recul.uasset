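; BP_Cell_Recul is a setback board cell that moves the player's pawn and applies a score penalty.
; Its Action override calls the parent, then has the game mode move the pawn to the current cell number plus NbCasesEnMoins and apply ScoreToRemove.
; It reports the sign-flipped offset to PlayerStatManager as cells travelled.
; The PlayerID input is unused, with ID 0 passed to the parent call and cell lookup.
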(event EventBeginPlay
  (|CallParentFunction) ; This node is disabled and will not be called.\nDrag off pins to build functionality.
)

(event Collision|EventActorBeginOverlap
  (params (OtherActor :type Actor%20Object%20Reference))
  (|CallParentFunction OtherActor) ; This node is disabled and will not be called.\nDrag off pins to build functionality.
)

(event EventTick
  (params (DeltaSeconds :type Float%20%28single-precision%29))
  (|CallParentFunction DeltaSeconds) ; This node is disabled and will not be called.\nDrag off pins to build functionality.
)

(fn ConstructionScript
  (|CallParentFunction))

(fn Action
  (params (PlayerID :type Integer))
  (bind _nbcasesenmoins (Variables|Default|GetNbCasesEnMoins))
  (bind _gmref (Variables|Default|GetGMRef))
  (|CallParentFunction 0)
  (bind _cellnumber (Default|GetPlayerCellNumberbyPlayerID (Variables|Default|GetGIRef)))
  (Default|MovePawn _gmref (+ _cellnumber _nbcasesenmoins))
  (Default|SetScorebyPlayerID _gmref (Variables|Default|GetScoreToRemove))
  (Class|PlayerStatsManager|NumberOfCellsTravelled (Variables|/Game/Blueprints/BP_GameMode.BP_GameMode_C|GetPlayerStatManager (Variables|Default|GetGMRef)) (* _nbcasesenmoins -1)))