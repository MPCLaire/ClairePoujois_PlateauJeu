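; BP_Cell_Forward is a board cell whose action pushes the player forward by a set number of cells.
; It overrides Action, calls the parent, then reads the player's current cell from the game instance reference and adds NbCasesEnPlus.
; Through the game mode reference it moves the pawn to that cell, applies ScoreToAdd to the score and reports the extra cells travelled to the PlayerStatManager.
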(event EventBeginPlay
  (|CallParentFunction) ; This node is disabled and will not be called.\nDrag off pins to build functionality.
)

(event Collision|EventActorBeginOverlap
  (params (OtherActor :type Actor%20Object%20Reference))
  (|CallParentFunction OtherActor) ; This node is disabled and will not be called.\nDrag off pins to build functionality.
)

(event EventTick
  (params (DeltaSeconds :type Float%20%28single-precision%29))
  (|CallParentFunction DeltaSeconds) ; This node is disabled and will not be called.\nDrag off pins to build functionality.
)

(fn ConstructionScript
  (|CallParentFunction))

(fn Action
  (params (PlayerID :type Integer))
  (bind _nbcasesenplus (Variables|Default|GetNbCasesEnPlus))
  (bind _gmref (Variables|Default|GetGMRef))
  (|CallParentFunction PlayerID)
  (bind _cellnumber (Default|GetPlayerCellNumberbyPlayerID (Variables|Default|GetGIRef) PlayerID))
  (Default|MovePawn _gmref (+ _cellnumber _nbcasesenplus))
  (Default|SetScorebyPlayerID _gmref (Variables|Default|GetScoreToAdd))
  (Class|PlayerStatsManager|NumberOfCellsTravelled (Variables|/Game/Blueprints/BP_GameMode.BP_GameMode_C|GetPlayerStatManager (Variables|Default|GetGMRef)) _nbcasesenplus))