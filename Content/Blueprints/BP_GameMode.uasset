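; Game mode for a two-player, turn-based dice board game that spawns both pawns, the dice and the roll widget.
; RollDice moves the current pawn by the dice result and triggers the landed cell's Action, or clamps it to the last cell and flags it finished.
; Player cell, score and end state live in BP_GameInstance.
; Turns cycle by modulo, skipping finished players' rolls, and pawns sharing a cell are nudged apart.
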(event EventBeginPlay
  (bind _asbp_game_instance (Utilities|Casting|CastToBP_GameInstance (Game|GetGameInstance)))
  (bind _output_get (Variables|Default|SetGIRef _asbp_game_instance))
  (Default|GetPlayerCellNumberbyPlayerID _output_get)
  (bind _returnvalue (Actor|GetActorOfClass "/Game/Blueprints/BP_Board.BP_Board_C"))
  (Variables|Default|SetBoardRef _returnvalue)
  (Utilities|FlowControl|Delay 0.1)
  (bind _cell_location (Default|GetCellPositionbyNumber (Variables|Default|GetBoardRef)))
  (bind _returnvalue_2 (Game|SpawnActorfromClass "/Game/Blueprints/BP_Pion.BP_Pion_C" (Math|Transform|MakeTransform _cell_location "0, 0, 0" "1.000000,1.000000,1.000000") "Undefined" "MultiplyWithRoot" 0 0))
  (Variables|Default|SetPionP1Ref _returnvalue_2)
  (bind _returnvalue_3 (Game|SpawnActorfromClass "/Game/Blueprints/BP_Pion2.BP_Pion2_C" (Math|Transform|MakeTransform _cell_location "0, 0, 0" "1.000000,1.000000,1.000000") "Undefined" "MultiplyWithRoot" 0 0))
  (Variables|Default|SetPionP2Ref _returnvalue_3)
  (CallFunction|CheckifPlayersonSameCell)
  (bind _returnvalue_4 (Game|SpawnActorfromClass "/Game/Blueprints/BP_Dice.BP_Dice_C" (Math|Transform|MakeTransform "0, 0, 0") "Undefined" "MultiplyWithRoot" 0 0))
  (Variables|Default|SetDiceRef _returnvalue_4)
  (CallFunction|SetPlayerIDbyPlayerRef)
  (bind _returnvalue_5 (UserInterface|CreateWidget "/Game/Widgets/WB_LancerDe.WB_LancerDe_C"))
  (UserInterface|Viewport|AddtoViewport _returnvalue_5 0)
  (Variables|Default|SetWidgetRef _returnvalue_5))

(event EventTick
  (params (DeltaSeconds :type Float%20%28single-precision%29)))

(fn ConstructionScript)

(fn RollDice
  (bind _diceref (Variables|Default|GetDiceRef))
  (bind _playerid (Variables|Default|GetPlayerID))
  (bind _playerid_2 (Variables|Default|GetPlayerID))
  (bind _giref (Variables|Default|GetGIRef))
  (bind _boardref (Variables|Default|GetBoardRef))
  (bind _celllist (Variables|/Game/Blueprints/BP_Board.BP_Board_C|GetCellList _boardref))
  (bind _playerlist (Variables|/Game/Blueprints/BP_GameInstance.BP_GameInstance_C|GetPlayerList _giref))
  (bind _returnvalue (Utilities|Array|Length _celllist))
  (bind _output (Utilities|Array|Get(acopy) _playerlist _playerid))
  (bind (_playerid_3 _score _cellnumber) (Utilities|Struct|BreakS_PlayerStruct _output))
  (bind _returnvalue_2 (- _returnvalue 1))
  (Default|SetScoreTextbyPlayerID (Variables|Default|GetWidgetRef) _playerid_2)
  (if (.IsAtEnd? (Utilities|Struct|BreakS_PlayerStruct (Utilities|Array|Get(acopy) (Variables|/Game/Blueprints/BP_GameInstance.BP_GameInstance_C|GetPlayerList (Variables|Default|GetGIRef)) _playerid_2)))
    (CallFunction|EndPlayerTurn)
    (else
      (Default|LaunchDice _diceref)
      (bind _cellnumber_2 (Default|GetPlayerCellNumberbyPlayerID (Variables|Default|GetGIRef) (Variables|Default|GetPlayerID)))
      ;[1 1 1] Définir quel joueur joue
      (bind _keys (Utilities|Map|Keys (Variables|Default|GetPlayerIDMap)))
      (Variables|Default|SetPionToPlay (Utilities|Array|Get(acopy) _keys (Variables|Default|GetPlayerID)))
      (if (< (+ _cellnumber_2 (Variables|/Game/Blueprints/BP_Dice.BP_Dice_C|GetDiceResult _diceref)) _returnvalue)
        (CallFunction|MovePawn (+ _cellnumber_2 (Variables|/Game/Blueprints/BP_Dice.BP_Dice_C|GetDiceResult _diceref)))
        (Default|Action (Utilities|Array|Get(acopy) (Variables|/Game/Blueprints/BP_Board.BP_Board_C|GetCellList (Variables|Default|GetBoardRef)) (+ _cellnumber_2 (Variables|/Game/Blueprints/BP_Dice.BP_Dice_C|GetDiceResult _diceref))) (Variables|Default|GetPlayerID))
        (else
          ;[1 1 1] Valider le fait que le pion est à la fin
          (Utilities|Array|SetArrayElem _playerlist _playerid (Utilities|Struct|MakeS_PlayerStruct _playerid_3 _score _cellnumber true))
          (Default|SetPlayerCellNumberbyPlayerID (Variables|Default|GetGIRef) (Variables|Default|GetPlayerID) _returnvalue_2)
          (CallFunction|MovePawn _returnvalue_2)))
      (CallFunction|CheckifPlayersonSameCell)
      ;[1 1 1] change le joueur qui joue
      (CallFunction|EndPlayerTurn))))

(fn SetPlayerIDbyPlayerRef
  ;[1 1 1] Donne un nombre int à un pion pour définir l'odre des joueurs
  (Variables|Default|SetPlayerIDMap (Utilities|Map|MakeMap (Variables|Default|GetPionP1Ref) (Variables|Default|GetPlayerID) (Variables|Default|GetPionP2Ref) (+ (Variables|Default|GetPlayerID) 1)))
  (Variables|Default|SetPlayerID 0))

(fn EndPlayerTurn
  (Variables|Default|SetPlayerID (Math|Integer|%(Integer) (+ (Variables|Default|GetPlayerID) 1) (Utilities|Map|Length (Variables|Default|GetPlayerIDMap)))))

(fn CheckifPlayersonSameCell
  (bind _giref (Variables|Default|GetGIRef))
  (bind _pionp2ref (Variables|Default|GetPionP2Ref))
  (bind _pionp1ref (Variables|Default|GetPionP1Ref))
  (bind _returnvalue (Transformation|GetActorLocation _pionp1ref))
  (bind _returnvalue_2 (Transformation|GetActorLocation _pionp2ref))
  (bind _playerlist (Variables|/Game/Blueprints/BP_GameInstance.BP_GameInstance_C|GetPlayerList _giref))
  ;[1 1 1] Vérifie qi les pions sont sur la même case et les décale un peu si c'est le cas
  (if (== (.CellNumber (Utilities|Struct|BreakS_PlayerStruct (Utilities|Array|Get(acopy) _playerlist))) (.CellNumber (Utilities|Struct|BreakS_PlayerStruct (Utilities|Array|Get(acopy) _playerlist 1))))
    (Transformation|SetActorLocation _pionp2ref (Math|Vector|MakeVector (.x _returnvalue_2) (+ (.y _returnvalue_2) 4e+01) (.z _returnvalue_2)) false false)
    (Transformation|SetActorLocation _pionp1ref (Math|Vector|MakeVector (.x _returnvalue) (- (.y _returnvalue) 4e+01) (.z _returnvalue)) false false)))

(fn MovePawn
  (params (CellIndex :type Integer))
  (Default|SetPlayerCellNumberbyPlayerID (Variables|Default|GetGIRef) (Variables|Default|GetPlayerID) CellIndex)
  (bind _cell_location (Default|GetCellPositionbyNumber (Variables|Default|GetBoardRef) CellIndex))
  (Default|MovetoNewCell (Variables|Default|GetPionToPlay) _cell_location))

(fn SetScorebyPlayerID
  (params (Score :type Integer))
  (bind _giref (Variables|Default|GetGIRef))
  (bind _playerid (Variables|Default|GetPlayerID))
  (bind _playerlist (Variables|/Game/Blueprints/BP_GameInstance.BP_GameInstance_C|GetPlayerList _giref))
  (bind _output (Utilities|Array|Get(acopy) _playerlist _playerid))
  (bind (_playerid_2 _score _cellnumber _isatend_) (Utilities|Struct|BreakS_PlayerStruct _output))
  (bind _output_get (Variables|Default|SetScore (+ Score (Variables|Default|GetScore))))
  (Utilities|Array|SetArrayElem _playerlist (Variables|Default|GetPlayerID) (Utilities|Struct|MakeS_PlayerStruct _playerid_2 _output_get _cellnumber _isatend_))
  (Default|SetScoreTextbyPlayerID (Variables|Default|GetWidgetRef) _playerid)
  (Variables|Default|SetScore 0))